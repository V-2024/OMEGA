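; BP_PatrolRoute is a spline-based patrol route for enemy AI that tracks the current patrol point.
; GetSplinPointAsWorldPosition returns the world location of the PatrolRoute spline point at PatrollIndex.
; IncrementPatrolRoute steps the index by Direction, flipping it at the first and last points so the route runs back and forth instead of looping.
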(event `IncrementPatrolRoute`
  (bind _output_get (set `self.PatrollIndex` (+ (`self.PatrollIndex`) (`self.Direction`))))
  (if (== _output_get (- (`SplineComponent.GetNumberOfSplinePoints` (`self.PatrolRoute`)) 1))
    (set `self.Direction` -1)
    (elif (== (`self.PatrollIndex`) 0)
      (set `self.Direction` 1))))

(fn `GetSplinPointAsWorldPosition`
  (returns (Location :type "Vector Structure"))
  (return (`SplineComponent.GetLocationAtSplinePoint` (`self.PatrolRoute`) (`self.PatrollIndex`) "World")))

(fn `UserConstructionScript`)