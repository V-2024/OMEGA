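; BP_Enemy_Ranged is a ranged enemy that fights with a rifle, extending a parent enemy Blueprint.
; On BeginPlay it spawns BP_Weapon_Rifle and attaches it to the right-hand socket.
; Attack plays the rifle fire montage, fires a damaging bullet through BPCAttacks on the montage notify, and ends on completion or interruption.
; It also maps movement states to walk speeds and reports long attack and defend radii.
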(event `self.ReceiveBeginPlay`
  (`parent.ReceiveBeginPlay`)
  (`/Game/SHJ/CustomContents/Enemies/AI/BPI_EnemyAI.EquipWeapon`))

(event `/Game/SHJ/CustomContents/Enemies/AI/BPI_EnemyAI.EquipWeapon`
  (bind _returnvalue (`|SpawnActorFromClass` "/Game/SHJ/CustomContents/Weapons/BP_Weapon_Rifle.BP_Weapon_Rifle_C" (`self.GetTransform`) "Undefined" "MultiplyWithRoot" null null))
  (bind _output_get (set `self.WeaponActor` _returnvalue))
  (`self.K2_AttachToComponent` _output_get (`self.Mesh`) "hand_r_rifle_socket" "SnapToTarget" "SnapToTarget" "SnapToTarget" true)
  (set `self.IsWieldingWeapon` true)
  (`self.OnEquipWeapon`))

(event `/Game/SHJ/CustomContents/Enemies/AI/BPI_EnemyAI.Attack`
  (params (AttackTarget :type "Actor Object Reference"))
  (`parent.Attack` AttackTarget)
  (bind _notifyname (`|PlayMontage` (`self.Mesh`) "/Game/SHJ/CustomContents/Animations/Rifle/Action/MM_Rifle_Fire_Montage.MM_Rifle_Fire_Montage")
    (:`OnCompleted`
      (`self.AttackEnd` AttackTarget :!label _label))
    (:`OnInterrupted`
      (goto _label))
    (:`OnNotifyBegin`
      (switch `name` _notifyname
        (:`Fire`
          (`/Game/SHJ/CustomContents/Attack/BPC_Attacks.FireBullet` (`self.BPC_Attacks`) (`self.K2_GetActorLocation` (`self.WeaponActor`)) (`self.K2_GetActorLocation` AttackTarget) (make `/Game/SHJ/CustomContents/DamageSystem/S_DamageInfo` 15.0 "NewEnumerator2")))))))

(fn `GetIdealRange`
  (returns (AttackRadius :type "Float (double-precision)") (DefendRadius :type "Float (double-precision)"))
  (return 2000.0 2000.0))

(fn `SetMovementSpeed`
  (params (Speed :type "/Game/SHJ/CustomContents/Enemies/AI/Enum/E_MovementSpeed Enum" :default "NewEnumerator0"))
  (returns (SpeedValue :type "Float (double-precision)"))
  (set `CharacterMovementComponent.MaxWalkSpeed` (select `/Game/SHJ/CustomContents/Enemies/AI/Enum/E_MovementSpeed` Speed :`NewEnumerator1` 100.0 :`NewEnumerator2` 300.0 :`NewEnumerator3` 500.0 :!type "Float (single-precision)") (`self.CharacterMovement`))
  (return 0.0))

(fn `UserConstructionScript`
  (`parent.UserConstructionScript`))